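; Main menu lighthouse-style light actor that plays audio on start and spins its light mesh while ShouldSpin is set.
; Tick applies frame-rate-scaled yaw rotation and turns the interact prompt on yaw only to face the player.
; It also defines helpers, uncalled within this Blueprint, to spawn boats at a random bearing or behind the light, targeting this actor, and to trigger LoseGame when a boat gets close.
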(event EventBeginPlay
  (Audio|Components|Audio|Play (Variables|Default|GetAudio) 0.0))

(event EventTick
  (params (DeltaSeconds :type Float%20%28single-precision%29))
  (Utilities|FlowControl|Sequence
    (:then_0
      (if (Variables|Default|GetShouldSpin)
        (CallFunction|SpinLight DeltaSeconds)))
    (:then_1
      (CallFunction|RotateTexttoPlayer))))

(fn ConstructionScript)

(fn SpinLight
  (params (DeltaTime :type Float%20%28double-precision%29))
  (bind _sm_light (Variables|Default|GetSM_Light))
  (bind _returnvalue (Transformation|GetWorldRotation _sm_light))
  (Transformation|AddWorldRotation _sm_light (Math|Rotator|MakeRotator 0.0 0.0 (* DeltaTime (Variables|Default|GetRotationRate))) false false)
  (if (>= (.yaw _returnvalue) 3.6e+02)
    (Transformation|SetWorldRotation _sm_light (Math|Rotator|MakeRotator 0.0 0.0 (- (.yaw _returnvalue) 3.6e+02)) false false)))

(fn RotateTexttoPlayer
  (bind _interactprompt (Variables|Default|GetInteractPrompt))
  (Transformation|SetWorldRotation _interactprompt (Math|Rotator|MakeRotator 0.0 0.0 (.yaw (Math|Rotator|FindLookatRotation (Transformation|GetWorldLocation _interactprompt) (Transformation|GetActorLocation (Game|GetPlayerCharacter 0))))) false false))

(fn SpawnBoat
  (bind _returnvalue (Transformation|GetActorLocation))
  (bind _returnvalue_2 (Math|Random|RandomUnitVector))
  (bind _returnvalue_3 (Math|Vector2D|MakeVector2D (.x _returnvalue_2) (.y _returnvalue_2)))
  (bind _returnvalue_4 (Class|KismetMathLibrary|NormalSafe2D _returnvalue_3 0.0))
  (bind _returnvalue_5 (* _returnvalue_4 1.2e+04))
  (bind _returnvalue_6 (+ _returnvalue _returnvalue_5))
  (bind _returnvalue_7 (Game|SpawnActorfromClass "/Game/Core/Blueprint/Lighthouse/BP_Boat.BP_Boat_C" (Math|Transform|MakeTransform (Math|Vector|MakeVector (.x _returnvalue_6) (.y _returnvalue_6) 3e+03) "0, 0, 0" "1.000000,1.000000,1.000000") "Undefined" "MultiplyWithRoot" 0 _returnvalue 0))
  (Variables|Default|SetBoat _returnvalue_7))

(fn SpawnMechanismBoat
  (bind _returnvalue (Transformation|GetActorLocation))
  (bind _sm_light (Variables|Default|GetSM_Light))
  (bind _returnvalue_2 (Math|Vector|GetForwardVector _sm_light))
  (bind _returnvalue_3 (* _returnvalue_2 -1.0))
  (bind _returnvalue_4 (* _returnvalue_3 1.2e+04))
  (bind _returnvalue_5 (+ _returnvalue_4 _returnvalue))
  (bind _returnvalue_6 (Game|SpawnActorfromClass "/Game/Core/Blueprint/Lighthouse/BP_Boat.BP_Boat_C" (Math|Transform|MakeTransform (Math|Vector|MakeVector (.x _returnvalue_5) (.y _returnvalue_5) 3e+03) "0, 0, 0" "1.000000,1.000000,1.000000") "Undefined" "MultiplyWithRoot" 0 _returnvalue 0))
  (Variables|Default|SetMechanismBoat _returnvalue_6))

(fn CheckBoatDistance
  (params (Boat :type Actor%20Object%20Reference))
  (Utilities|IsValid Boat
    (:Is%20Valid
      (if (<= (Math|Vector|Distance(Vector) (Transformation|GetActorLocation Boat) (Transformation|GetActorLocation)) 4e+03)
        (Default|LoseGame (Variables|Default|GetPlayerController))))))