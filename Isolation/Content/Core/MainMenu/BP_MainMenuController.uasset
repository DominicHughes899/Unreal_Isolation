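; BP_MainMenuController is the main menu player controller, showing the menu and handling the transition into the game.
; BeginPlay adds the menu and fade widgets to the viewport and shows the cursor.
; StartGame_Event switches to game-only input, starts the widget's fade-out and opens L_Main after a delay.
; Meanwhile, Tick lerps the Master sound class volume to silence through a sound mix override.
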(event Custom|Start%20Game_Event
  (Variables|Default|SetShould%20Fade%20out true)
  (Input|SetInputModeGameOnly self false)
  (Variables|Default|SetbShowMouseCursor false)
  (Default|FadeOut (Variables|Default|GetFadeInUI))
  (Utilities|FlowControl|Delay 5.0)
  (Game|OpenLevel(byName) "L_Main"))

(event EventBeginPlay
  (bind _returnvalue (UserInterface|CreateWidget "/Game/Core/MainMenu/Widgets/WBP_MainMenu.WBP_MainMenu_C"))
  (bind _output_get (Variables|Default|SetUI _returnvalue))
  (UserInterface|Viewport|AddtoViewport _output_get 0)
  (bind _returnvalue_2 (UserInterface|CreateWidget "/Game/Core/MainMenu/Widgets/WBP_FadeIn.WBP_FadeIn_C"))
  (bind _output_get_2 (Variables|Default|SetFadeInUI _returnvalue_2))
  (UserInterface|Viewport|AddtoViewport _output_get_2 0)
  (Variables|Default|SetbShowMouseCursor true))

(event EventTick
  (params (DeltaSeconds :type Float%20%28single-precision%29))
  (if (Variables|Default|GetShould%20Fade%20out)
    (bind _output_get (Variables|Default|SetFadeTimer (+ DeltaSeconds (Variables|Default|GetFadeTimer))))
    (Audio|SetSoundMixClassOverride "/Game/Core/Audio/Mix_Main.Mix_Main" "/Engine/EngineSounds/Master.Master" (Math|Float|Lerp 1.0 0.0 (/ _output_get 3.0)) 1.0 0.0 true)))

(fn ConstructionScript)

(fn PlayLevel)