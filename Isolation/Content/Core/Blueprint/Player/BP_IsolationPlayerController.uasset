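; Player controller that runs a match's flow and HUD: a paused intro, relic collection, and win or lose screens.
; BeginPlay creates the HUD and start overlays, then after a delay unpauses, starts the score timer and fades in master volume on Tick through a sound mix override.
; Events update relic count, fuel bar and mechanism warning; reaching the relic target wins, and both endings pause and show the elapsed time.
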(event Custom|Update%20Relics
  (bind _result (Math|Integer|IncrementInt (Variables|Default|GetRelicCounter))
    (:%20%20
      (Variables|/Script/UMG.TextBlock|SetText (Variables|/Game/Core/UI/WBP_Overlay.WBP_Overlay_C|GetRelicCounter (Variables|Default|GetOverlay)) (Utilities|Text|ToText(Integer) _result))
      (if (== (Variables|Default|GetRelicCounter) 6)
        (CallFunction|WinGame)))))

(event Custom|Lose%20Game
  (Audio|PlaySound2D "/Game/Core/Audio/SFX/Cues/SC_Impact.SC_Impact" 1.0 1.0 0.0 0 0)
  (Game|SetGamePaused true)
  (bind _returnvalue (UserInterface|CreateWidget "/Game/Core/UI/Misc/WBP_LoseScreen.WBP_LoseScreen_C" 0 (Math|Conversions|ToFloat(Integer) (Math|Float|Round (Variables|Default|GetScoreTimer)))))
  (UserInterface|Viewport|AddtoViewport _returnvalue 0)
  (Input|SetInputModeUIOnly self 0 "DoNotLock" false)
  (Variables|Default|SetbShowMouseCursor true))

(event Custom|Win%20Game
  (Game|SetGamePaused true)
  (bind _returnvalue (UserInterface|CreateWidget "/Game/Core/UI/Misc/WBP_WinScreen.WBP_WinScreen_C" 0 (Math|Conversions|ToFloat(Integer) (Math|Float|Round (Variables|Default|GetScoreTimer)))))
  (UserInterface|Viewport|AddtoViewport _returnvalue 0)
  (Input|SetInputModeUIOnly self 0 "DoNotLock" false)
  (Variables|Default|SetbShowMouseCursor true))

(event Custom|UpdateMechanismWarning_Event
  (params (ShowWarning :type Boolean))
  (bind _overlay (Variables|Default|GetOverlay))
  (bind _mechanismwarning (Variables|/Game/Core/UI/WBP_Overlay.WBP_Overlay_C|GetMechanismWarning _overlay))
  (if ShowWarning
    (Widget|SetVisibility _mechanismwarning "Visible")
    (else
      (Widget|SetVisibility _mechanismwarning "Hidden"))))

(event EventBeginPlay
  (Input|SetInputModeGameOnly self false)
  (Game|SetGamePaused true)
  (bind _returnvalue (UserInterface|CreateWidget "/Game/Core/UI/WBP_Overlay.WBP_Overlay_C"))
  (bind _output_get (Variables|Default|SetOverlay _returnvalue))
  (UserInterface|Viewport|AddtoViewport _output_get 0)
  (bind _returnvalue_2 (UserInterface|CreateWidget "/Game/Core/UI/Misc/WBP_StartOverlay.WBP_StartOverlay_C"))
  (UserInterface|Viewport|AddtoViewport _returnvalue_2 0)
  (Utilities|FlowControl|Delay 6.0)
  (Variables|Default|SetShouldFadeSoundIn true)
  (Game|SetGamePaused false)
  (Variables|Default|SetShouldCount true))

(event EventTick
  (params (DeltaSeconds :type Float%20%28single-precision%29))
  (Utilities|FlowControl|Sequence
    (:then_0
      (if (Variables|Default|GetShouldCount)
        (Variables|Default|SetScoreTimer (+ DeltaSeconds (Variables|Default|GetScoreTimer)))))
    (:then_1
      (if (Variables|Default|GetShouldFadeSoundIn)
        (bind _output_get (Variables|Default|SetSoundFadeTimer (+ DeltaSeconds (Variables|Default|GetSoundFadeTimer))))
        (Audio|SetSoundMixClassOverride "/Game/Core/Audio/Mix_Main.Mix_Main" "/Engine/EngineSounds/Master.Master" (/ _output_get 3.0) 1.0 0.0 true)
        (if (>= (/ _output_get 3.0) 1.0)
          (Variables|Default|SetSoundFadeTimer 0.0)
          (Variables|Default|SetShouldFadeSoundIn false))))))

(fn ConstructionScript)

(fn UpdateFuelUI
  (params (NewPercent :type Float%20%28double-precision%29))
  (Variables|/Game/Core/UI/WBP_Overlay.WBP_Overlay_C|SetFuelbarPercent (Variables|Default|GetOverlay) NewPercent))