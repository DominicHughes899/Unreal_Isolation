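; BP_MasterRelic is a relic pickup, apparently the base for relics, that animates in the world and reports to the player controller.
; Tick spins and sine-bobs the mesh and yaws the prompt toward the player.
; OnFocus and OnUnfocus toggle the prompt, with a discovery sound, primed at BeginPlay, playing on first focus.
; OnDestroy calls UpdateRelics on the cached BP_IsolationPlayerController and prints a debug string.
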(event EventBeginPlay
  (bind _asbp_isolation_player_controller (Utilities|Casting|CastToBP_IsolationPlayerController (Game|GetPlayerController 0)))
  (Variables|Default|SetPlayerController _asbp_isolation_player_controller)
  (Class|GameplayStatics|PrimeSound "/Game/Core/Audio/SFX/Cues/SC_Discovery.SC_Discovery"))

(event EventTick
  (params (DeltaSeconds :type Float%20%28single-precision%29))
  (CallFunction|Spin DeltaSeconds)
  (CallFunction|Bounce DeltaSeconds)
  (CallFunction|RotateTexttoPlayer))

(event EventOnFocus
  (Rendering|SetVisibility (Variables|Default|GetPrompt) true false)
  (Utilities|FlowControl|DoOnce false
    (:Completed
      (Audio|PlaySound2D "/Game/Core/Audio/SFX/Cues/SC_Discovery.SC_Discovery" 1.0 1.0 0.0 0 0))))

(event EventOnUnfocus
  (Rendering|SetVisibility (Variables|Default|GetPrompt) false false))

(event EventOnDestroy
  (Default|UpdateRelics (Variables|Default|GetPlayerController))
  (Development|PrintString "Hello"))

(fn ConstructionScript)

(fn Spin
  (params (DT :type Float%20%28double-precision%29))
  (bind _relicmesh (Variables|Default|GetRelicMesh))
  (bind _returnvalue (Transformation|GetWorldRotation _relicmesh))
  (Transformation|AddWorldRotation _relicmesh (Math|Rotator|MakeRotator 0.0 0.0 (* DT (Variables|Default|GetAnimSpinRate))) false false)
  (if (>= (.yaw _returnvalue) 3.6e+02)
    (Transformation|SetWorldRotation _relicmesh (Math|Rotator|MakeRotator 0.0 0.0 (- (.yaw _returnvalue) 3.6e+02)) false false)))

(fn Bounce
  (params (DT :type Float%20%28double-precision%29))
  (bind _output_get (Variables|Default|SetBounce%20Timer (+ DT (Variables|Default|GetBounce%20Timer))))
  (Transformation|AddWorldOffset (Variables|Default|GetRelicMesh) (Math|Vector|MakeVector 0.0 0.0 (/ (Math|Trig|Sin(Radians) (* _output_get 2.0)) 2.0)) false false))

(fn RotateTexttoPlayer
  (Transformation|SetWorldRotation (Variables|Default|GetPrompt) (Math|Rotator|MakeRotator 0.0 0.0 (.yaw (Math|Rotator|FindLookatRotation (Transformation|GetActorLocation) (Transformation|GetActorLocation (Game|GetPlayerCharacter 0))))) false false))