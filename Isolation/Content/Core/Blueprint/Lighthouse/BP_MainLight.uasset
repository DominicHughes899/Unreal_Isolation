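; Lighthouse main light that spins and burns fuel, losing the game when a boat gets too close.
; Running out of fuel darkens the spotlight and spawns a boat around the lighthouse; stopping the mechanism spawns another opposite the beam.
; Refuelling or restarting kills the matching boat, while Tick checks boat distances.
; It also updates fuel and warning UI via the player controller and shows a player-facing interaction prompt on focus.
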(event Custom|StopSpinning_Event
  ;[1 1 1] Mechanism
  (Variables|Default|SetShouldSpin false)
  (CallFunction|SpawnMechanismBoat)
  (Variables|Default|SetIsMechanismBoatComing true)
  (Default|UpdateMechanismWarningEvent (Variables|Default|GetPlayerController) true))

(event Custom|RestartSpinning_Event
  ;[1 1 1] Mechanism
  (Variables|Default|SetShouldSpin true)
  (Default|Kill (Variables|Default|GetMechanismBoat))
  (Variables|Default|SetIsMechanismBoatComing false)
  (Default|UpdateMechanismWarningEvent (Variables|Default|GetPlayerController) false))

(event EventBeginPlay
  (bind _asbp_isolation_player_controller (Utilities|Casting|CastToBP_IsolationPlayerController (Game|GetPlayerController 0)))
  (Variables|Default|SetPlayerController _asbp_isolation_player_controller))

(event EventOnFuelEmpty
  ;[1 1 1] Fueling
  (Rendering|Components|Light|SetIntensity (Variables|Default|GetSpotLight) 0.0)
  (CallFunction|SpawnBoat)
  (Variables|Default|SetIsBoatComing true))

(event EventTick
  (params (DeltaSeconds :type Float%20%28single-precision%29))
  (Utilities|FlowControl|Sequence
    (:then_0
      (if (Variables|Default|GetShouldSpin)
        (CallFunction|SpinLight DeltaSeconds)))
    (:then_1
      (CallFunction|RotateTexttoPlayer))
    (:then_2
      (if (Variables|Default|GetIsBoatComing)
        (CallFunction|CheckBoatDistance (Variables|Default|GetBoat))))
    (:then_3
      (if (Variables|Default|GetIsMechanismBoatComing)
        (CallFunction|CheckBoatDistance (Variables|Default|GetMechanismBoat))))))

(event EventOnFocus
  (params (HasFuel :type Boolean))
  (bind _interactprompt (Variables|Default|GetInteractPrompt))
  ;[1 1 1] Focus
  (Rendering|SetVisibility _interactprompt true false)
  (if HasFuel
    (Rendering|Components|TextRender|SetText _interactprompt (Utilities|Text|MakeLiteralText "Fill"))
    (Rendering|Components|TextRender|SetTextRenderColor _interactprompt (Math|Color|MakeColor 255 255 255 255))
    (else
      (Rendering|Components|TextRender|SetText _interactprompt (Utilities|Text|MakeLiteralText "Need Fuel"))
      (Rendering|Components|TextRender|SetTextRenderColor _interactprompt (Math|Color|MakeColor 0 0 255 255)))))

(event EventOnUnfocus
  ;[1 1 1] Focus
  (Rendering|SetVisibility (Variables|Default|GetInteractPrompt) false false))

(event EventOnDrainFuel
  (params (CurrentLevel :type Float%20%28single-precision%29))
  ;[1 1 1] Fueling
  ;;[0 0.008149 1] UI
  (Default|UpdateFuelUI (Variables|Default|GetPlayerController) CurrentLevel))

(event EventOnFuelRefill
  ;[1 1 1] Fueling
  (Rendering|Components|Light|SetIntensity (Variables|Default|GetSpotLight) 8.8e+02)
  (Default|Kill (Variables|Default|GetBoat))
  (Variables|Default|SetIsBoatComing false))

(fn ConstructionScript)

(fn SpinLight
  (params (DeltaTime :type Float%20%28double-precision%29))
  (bind _sm_light (Variables|Default|GetSM_Light))
  (bind _returnvalue (Transformation|GetWorldRotation _sm_light))
  (Transformation|AddWorldRotation _sm_light (Math|Rotator|MakeRotator 0.0 0.0 (* DeltaTime (Variables|Default|GetRotationRate))) false false)
  (if (>= (.yaw _returnvalue) 3.6e+02)
    (Transformation|SetWorldRotation _sm_light (Math|Rotator|MakeRotator 0.0 0.0 (- (.yaw _returnvalue) 3.6e+02)) false false)))

(fn RotateTexttoPlayer
  (bind _interactprompt (Variables|Default|GetInteractPrompt))
  (Transformation|SetWorldRotation _interactprompt (Math|Rotator|MakeRotator 0.0 0.0 (.yaw (Math|Rotator|FindLookatRotation (Transformation|GetWorldLocation _interactprompt) (Transformation|GetActorLocation (Game|GetPlayerCharacter 0))))) false false))

(fn SpawnBoat
  (bind _returnvalue (Transformation|GetActorLocation))
  (bind _returnvalue_2 (Math|Random|RandomUnitVector))
  (bind _returnvalue_3 (Math|Vector2D|MakeVector2D (.x _returnvalue_2) (.y _returnvalue_2)))
  (bind _returnvalue_4 (Class|KismetMathLibrary|NormalSafe2D _returnvalue_3 0.0))
  (bind _returnvalue_5 (* _returnvalue_4 1.2e+04))
  (bind _returnvalue_6 (+ _returnvalue _returnvalue_5))
  (bind _returnvalue_7 (Game|SpawnActorfromClass "/Game/Core/Blueprint/Lighthouse/BP_Boat.BP_Boat_C" (Math|Transform|MakeTransform (Math|Vector|MakeVector (.x _returnvalue_6) (.y _returnvalue_6) 3e+03) "0, 0, 0" "1.000000,1.000000,1.000000") "Undefined" "MultiplyWithRoot" 0 _returnvalue 0))
  (Variables|Default|SetBoat _returnvalue_7))

(fn SpawnMechanismBoat
  (bind _returnvalue (Transformation|GetActorLocation))
  (bind _sm_light (Variables|Default|GetSM_Light))
  (bind _returnvalue_2 (Math|Vector|GetForwardVector _sm_light))
  (bind _returnvalue_3 (* _returnvalue_2 -1.0))
  (bind _returnvalue_4 (* _returnvalue_3 1.2e+04))
  (bind _returnvalue_5 (+ _returnvalue_4 _returnvalue))
  (bind _returnvalue_6 (Game|SpawnActorfromClass "/Game/Core/Blueprint/Lighthouse/BP_Boat.BP_Boat_C" (Math|Transform|MakeTransform (Math|Vector|MakeVector (.x _returnvalue_5) (.y _returnvalue_5) 3e+03) "0, 0, 0" "1.000000,1.000000,1.000000") "Undefined" "MultiplyWithRoot" 0 _returnvalue 0))
  (Variables|Default|SetMechanismBoat _returnvalue_6))

(fn CheckBoatDistance
  (params (Boat :type Actor%20Object%20Reference))
  (bind _returnvalue (Transformation|GetActorLocation Boat))
  (Utilities|IsValid Boat
    (:Is%20Valid
      (if (<= (Math|Vector|Distance(Vector) _returnvalue (Transformation|GetActorLocation)) 5e+03)
        (Audio|SpawnSoundatLocation "/Game/Core/Audio/SFX/Cues/SC_Impact.SC_Impact" _returnvalue "0, 0, 0" 1.0 1.0 0.0 0 0)
        (Default|LoseGame (Variables|Default|GetPlayerController))))))