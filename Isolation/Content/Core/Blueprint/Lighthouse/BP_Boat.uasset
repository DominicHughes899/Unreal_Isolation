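; BP_Boat is a lighthouse boat actor that sails in a straight line while playing an attached fog horn sound.
; On BeginPlay it starts the horn on the ship mesh and rotates its root to face TargetLocation.
; Each tick it moves along local forward by Speed, with no delta-time scaling or sweep.
; A Kill function stops the sound and destroys the actor.
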(event EventBeginPlay
  (bind _returnvalue (Audio|SpawnSoundAttached "/Game/Core/Audio/SFX/Cues/SC_FogHorn.SC_FogHorn" (Variables|Default|GetSM_Ship) "None" "0, 0, 0" "0, 0, 0" "KeepRelativeOffset" false 1.0 1.0 0.0 0 0))
  (bind _output_get (Variables|Default|SetSound%20comp _returnvalue))
  (Audio|Components|Audio|Play _output_get 0.0)
  (Transformation|SetWorldRotation (Variables|Default|GetDefaultSceneRoot) (Math|Rotator|FindLookatRotation (Transformation|GetActorLocation) (Variables|Default|GetTargetLocation)) false false))

(event EventTick
  (params (DeltaSeconds :type Float%20%28single-precision%29))
  (Transformation|AddActorLocalOffset (* (Math|Vector|GetForwardVector "0, 0, 0") (Variables|Default|GetSpeed)) false false))

(fn ConstructionScript)

(fn Kill
  (Audio|Components|Audio|Stop (Variables|Default|GetSound%20comp))
  (Actor|DestroyActor))