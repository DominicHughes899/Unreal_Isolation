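; BP_FuelCan is a lighthouse fuel can prop that animates in the world and carries an interact prompt facing the player.
; While ShouldAnimate is set, Tick spins the mesh around yaw at AnimSpinRate and bobs it with a sine-driven world offset.
; The same Tick turns InteractPrompt toward player 0 using only the yaw of a look-at rotation.
; The graphs contain no pickup or interaction logic.
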(event EventBeginPlay)

(event EventTick
  (params (DeltaSeconds :type Float%20%28single-precision%29))
  (if (Variables|Default|GetShouldAnimate)
    (CallFunction|SpinAnimation DeltaSeconds)
    (CallFunction|BounceAnimation DeltaSeconds)
    (CallFunction|RotateTexttoPlayer)))

(fn ConstructionScript)

(fn SpinAnimation
  (params (DT :type Float%20%28double-precision%29))
  (bind _sm_gas_can (Variables|Default|GetSM_gas_can))
  (bind _returnvalue (Transformation|GetWorldRotation _sm_gas_can))
  (Transformation|AddWorldRotation _sm_gas_can (Math|Rotator|MakeRotator 0.0 0.0 (* DT (Variables|Default|GetAnimSpinRate))) false false)
  (if (>= (.yaw _returnvalue) 3.6e+02)
    (Transformation|SetWorldRotation _sm_gas_can (Math|Rotator|MakeRotator 0.0 0.0 (- (.yaw _returnvalue) 3.6e+02)) false false)))

(fn BounceAnimation
  (params (DT :type Float%20%28double-precision%29))
  (bind _output_get (Variables|Default|SetBounceTimer (+ DT (Variables|Default|GetBounceTimer))))
  (Transformation|AddWorldOffset (Variables|Default|GetSM_gas_can) (Math|Vector|MakeVector 0.0 0.0 (/ (Math|Trig|Sin(Radians) (* _output_get 2.0)) 2.0)) false false))

(fn RotateTexttoPlayer
  (Transformation|SetWorldRotation (Variables|Default|GetInteractPrompt) (Math|Rotator|MakeRotator 0.0 0.0 (.yaw (Math|Rotator|FindLookatRotation (Transformation|GetActorLocation) (Transformation|GetActorLocation (Game|GetPlayerCharacter 0))))) false false))