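; BP_LighthouseMechanism is a lighthouse mechanism actor that owns spinning gears and shows a prompt when focused.
; On BeginPlay it casts its child actor to BP_SpinningGears and stores it as OwnedGears.
; Focus and unfocus events toggle the prompt's visibility.
; Every tick, the prompt is rotated in yaw only to face the player character, keeping the text upright.
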(event EventBeginPlay
  (bind _asbp_spinning_gears (Utilities|Casting|CastToBP_SpinningGears (Variables|/Script/Engine.ChildActorComponent|GetChildActor (Variables|Default|GetChildActor))))
  (Variables|Default|SetOwnedGears _asbp_spinning_gears))

(event EventOnFocus
  (Rendering|SetVisibility (Variables|Default|GetPrompt) true false))

(event EventOnUnfocus
  (Rendering|SetVisibility (Variables|Default|GetPrompt) false false))

(event EventTick
  (params (DeltaSeconds :type Float%20%28single-precision%29))
  (CallFunction|RotateTexttoPlayer))

(fn ConstructionScript)

(fn RotateTexttoPlayer
  (Transformation|SetWorldRotation (Variables|Default|GetPrompt) (Math|Rotator|MakeRotator 0.0 0.0 (.yaw (Math|Rotator|FindLookatRotation (Transformation|GetWorldLocation (Variables|Default|GetPrompt)) (Transformation|GetActorLocation (Game|GetPlayerCharacter 0))))) false false))